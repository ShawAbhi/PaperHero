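; Lobby pawn that tracks device screen orientation and rolls its camera to match.
; Each tick on the local pawn, it classifies the motion-sensor gravity yaw into portrait or landscape variants, always using Portrait on Windows.
; On a change, it waits briefly, plays a timeline meant to lerp camera roll, and broadcasts orientation and viewport size on the Input.Orientation gameplay message channel.
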(event Custom|OnOrientaionChanged
  (params (Orientation :type EScreenOrientation%20Enum :default "Unknown"))
  (Utilities|FlowControl|Delay 0.2)
  (CallFunction|UpdateCameraOrientation Orientation)
  (Messaging|BroadcastMessage (Subsystems|GetGameplayMessageSubsystem) "(TagName=\"Input.Orientation\")" (Utilities|Struct|MakeFOrientation Orientation (Viewport|GetViewportSize))))

(event EventBeginPlay)

(event Collision|EventActorBeginOverlap
  (params (OtherActor :type Actor%20Object%20Reference)))

(event EventTick
  (params (DeltaSeconds :type Float%20%28single-precision%29))
  (CallFunction|UpdateOrientation))

(fn ConstructionScript)

(fn UpdateCameraOrientation
  (params (Orientation :type EScreenOrientation%20Enum :default "Unknown"))
  (bind _output_get (Variables|Default|SetA_TempCameraRot (Variables|/Script/Engine.SceneComponent|GetRelativeRotation (Variables|Default|GetCamera1))))
  (Variables|Default|SetB_TempCameraRot (Math|Rotator|MakeRotator (Utilities|Select :Index Orientation :Unknown 0.0 :Portrait 0.0 :PortraitUpsideDown 1.8e+02 :LandscapeLeft 2.7e+02 :LandscapeRight 9e+01 :FaceUp 0.0 :FaceDown 0.0 :PortraitSensor 0.0 :LandscapeSensor 0.0 :FullSensor 0.0) (.Pitch (Math|Rotator|BreakRotator _output_get)) (.Yaw (Math|Rotator|BreakRotator _output_get))))
  (Components|Timeline|PlayfromStart (Variables|Default|GetOrientationChange)))

(fn UpdateOrientation
  (if (Pawn|IsLocallyControlled)
    (Utilities|FlowControl|Sequence
      (:then_0
        (if (not (Class|LowEntryExtendedStandardLibrary|WindowsPlatform))
          (Variables|Default|SetCachedRotation (.yaw (Math|Rotator|MakeRotfromX (.Gravity (Class|PlayerController|GetInputMotionState (Game|GetPlayerController 0))))))
          (if (Math|Float|InRange(Float) (Variables|Default|GetCachedRotation) 6e+01 1.2e+02)
            (Variables|Default|SetOrientation "Portrait")
            (elif (Math|Float|InRange(Float) (Variables|Default|GetCachedRotation) -3e+01 3e+01)
              (Variables|Default|SetOrientation "LandscapeLeft")
              (elif (Math|Float|InRange(Float) (Variables|Default|GetCachedRotation) -1.2e+02 -6e+01)
                (Variables|Default|SetOrientation "PortraitUpsideDown")
                (elif (or (Math|Float|InRange(Float) (Variables|Default|GetCachedRotation) -1.9e+02 -1.5e+02) (Math|Float|InRange(Float) (Variables|Default|GetCachedRotation) 1.5e+02 1.9e+02))
                  (Variables|Default|SetOrientation "LandscapeRight")))))
          (else
            (Variables|Default|SetOrientation "Portrait"))))
      (:then_1
        (if (Utilities|Enum|NotEqual(Enum) (Variables|Default|GetPrevOrientation) (Variables|Default|GetOrientation))
          (Variables|Default|SetPrevOrientation (Variables|Default|GetOrientation))
          (CallFunction|OnOrientaionChanged (Variables|Default|GetOrientation)))))))