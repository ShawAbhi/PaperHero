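; Base sprite character that moves and jumps via keyboard axes or a virtual touch joystick with double-tap jump, flipping its sprite to face movement.
; Tick feeds touch drag into orientation-adjusted movement and passes stick endpoints to the HUD for drawing.
; Gravity-based orientation detection is immediately overridden to Portrait; orientation changes update a test widget and start a camera-roll timeline.
; That widget's value also sets spring arm length.
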(event Custom|DoubleTap
  ;[1 1 1] PC controls
  (Character|Jump))

(event Custom|MoveForward
  (params (ScaleValue :type Float%20%28single-precision%29))
  (bind _orientation (Variables|Default|GetOrientation))
  (bind _returnvalue (Utilities|Select :Index _orientation :Unknown 1.0 :Portrait 1.0 :PortraitUpsideDown -1.0 :LandscapeLeft 1.0 :LandscapeRight -1.0 :FaceUp 1.0 :FaceDown 1.0 :PortraitSensor 1.0 :LandscapeSensor 1.0 :FullSensor 1.0))
  (bind _returnvalue_2 (* ScaleValue _returnvalue))
  (Pawn|Input|AddMovementInput "0.000000,-1.000000,0.000000" _returnvalue_2 false)
  (Utilities|FlowControl|Gate true
    (:Exit
      (CallFunction|UpdateSpriteDirection _returnvalue_2))))

(event Custom|MoveRight
  (params (ScaleValue :type Float%20%28single-precision%29))
  (bind _orientation (Variables|Default|GetOrientation))
  (bind _returnvalue (Utilities|Select :Index _orientation :Unknown 1.0 :Portrait 1.0 :PortraitUpsideDown -1.0 :LandscapeLeft -1.0 :LandscapeRight 1.0 :FaceUp 1.0 :FaceDown 1.0 :PortraitSensor 1.0 :LandscapeSensor 1.0 :FullSensor 1.0))
  (bind _returnvalue_2 (* ScaleValue _returnvalue))
  (Pawn|Input|AddMovementInput "1.000000,0.000000,0.000000" _returnvalue_2 false)
  (bind _bool (CallFunction|UpdateSpriteDirection _returnvalue_2))
  (if _bool
    (Utilities|FlowControl|Gate true) ; enters at Close
    (else
      (Utilities|FlowControl|Gate true) ; enters at Open
    )))

(event Custom|UpdateTouchControls
  (bind _returnvalue (Game|GetPlayerController 0))
  (bind _as_bp_base_hud (Variables|Default|GetAs%20BP%20Base%20Hud))
  (bind _orientation (Variables|Default|GetOrientation))
  (bind (_locationx _locationy _biscurrentlypressed) (Class|PlayerController|GetInputTouchState _returnvalue "Touch1"))
  (bind _returnvalue_2 (Utilities|Enum|Equal(Enum) _orientation "LandscapeLeft"))
  (bind _returnvalue_3 (Utilities|Enum|Equal(Enum) _orientation "LandscapeRight"))
  (bind _returnvalue_4 (or _returnvalue_2 _returnvalue_3))
  ;[1 1 1] Touch
  (if (== (Pawn|GetControlledPawn _returnvalue) self)
    (if _biscurrentlypressed
      (Variables|Default|SetCurrentTouchLocation (Math|Vector|MakeVector _locationx _locationy 0.0))
      (if (Variables|Default|GetFirstTap)
        (Utilities|FlowControl|Sequence
          (:then_0
            (Utilities|IsValid _as_bp_base_hud
              (:Is%20Valid
                (Variables|/Game/Blueprints/GamePlay/BP_BaseHud.BP_BaseHud_C|SetDrawLineStart _as_bp_base_hud (Variables|Default|GetStartTouchLocation))
                (Variables|/Game/Blueprints/GamePlay/BP_BaseHud.BP_BaseHud_C|SetDrawLineEnd _as_bp_base_hud (Variables|Default|GetCurrentTouchLocation)))))
          (:then_1
            (if (> (Math|Vector|Distance2D(Vector) (Variables|Default|GetStartTouchLocation) (Variables|Default|GetCurrentTouchLocation)) 1.5e+02)
              (Variables|Default|SetStartTouchLocation (- (Variables|Default|GetCurrentTouchLocation) (* (Math|Vector|GetForwardVector (Math|Rotator|FindLookatRotation (Variables|Default|GetStartTouchLocation) (Variables|Default|GetCurrentTouchLocation))) 1.5e+02)))))
          (:then_2
            (if (> (Math|Vector|Distance2D(Vector) (Variables|Default|GetStartTouchLocation) (Variables|Default|GetCurrentTouchLocation)) 15.0)
              (CallFunction|MoveRight (select _returnvalue_4 (Math|Float|Clamp(Float) (/ (.Y (Math|Vector|BreakVector (- (Variables|Default|GetStartTouchLocation) (Variables|Default|GetCurrentTouchLocation)))) 1.3e+02) -1.0) (Math|Float|Clamp(Float) (/ (* (.X (Math|Vector|BreakVector (- (Variables|Default|GetStartTouchLocation) (Variables|Default|GetCurrentTouchLocation)))) -1.0) 1e+02) -1.0)))
              (CallFunction|MoveForward (select _returnvalue_4 (Math|Float|Clamp(Float) (/ (* (.X (Math|Vector|BreakVector (- (Variables|Default|GetStartTouchLocation) (Variables|Default|GetCurrentTouchLocation)))) -1.0) 1e+02) -1.0) (Math|Float|Clamp(Float) (/ (.Y (Math|Vector|BreakVector (- (Variables|Default|GetStartTouchLocation) (Variables|Default|GetCurrentTouchLocation)))) 1.3e+02) -1.0))))))
        (else
          (Variables|Default|SetFirstTap true)
          (Variables|Default|SetStartTouchLocation (Variables|Default|GetCurrentTouchLocation))
          (Utilities|FlowControl|Sequence
            (:then_0
              (if (Variables|Default|GetbIsDoubleTap)
                (Variables|Default|SetbIsDoubleTap false)
                (CallFunction|DoubleTap)
                (else
                  (Variables|Default|SetbIsDoubleTap true)
                  (Utilities|FlowControl|Delay (Variables|Default|GetDoubleTapCooldown))
                  (Variables|Default|SetbIsDoubleTap false)))))))
      (else
        (Variables|Default|SetFirstTap false)))))

(event Custom|ToggleCameraState
  (params (Portrait :type Boolean))
  (bind _springarm (Variables|Default|GetSpringArm))
  (if Portrait
    (Variables|/Script/Engine.SpringArmComponent|SetTargetArmLength _springarm 1.3e+03)
    (else
      (Variables|/Script/Engine.SpringArmComponent|SetTargetArmLength _springarm 6e+02))))

(event Custom|ValueUpdated
  (params (Value :type Float%20%28double-precision%29))
  (Variables|/Script/Engine.SpringArmComponent|SetTargetArmLength (Variables|Default|GetSpringArm) Value))

(event Custom|OnOrientaionChanged
  (params (Orientation :type EScreenOrientation%20Enum :default "Unknown"))
  (Development|PrintString (Utilities|String|EnumtoString Orientation) true false)
  (CallFunction|UpdateCameraOrientation Orientation)
  (Default|OnOrientationChanged (Variables|Default|GetTestUI) Orientation))

(event EventBeginPlay
  (Utilities|FlowControl|Sequence
    (:then_0
      (bind _returnvalue (UserInterface|CreateWidget "/Game/Blueprints/UI/MasterUIs/WBP_ScalarTest.WBP_ScalarTest_C"))
      (UserInterface|Viewport|AddtoViewport _returnvalue 0)
      (bind _output_get (Variables|Default|SetTestUI _returnvalue))
      (EventDispatchers|BindEventtoValueUpdated _output_get (delegate Custom|ValueUpdated)))
    (:then_1
      (bind _asbp_base_hud (Utilities|Casting|CastToBP_BaseHud (HUD|GetHUD (Game|GetPlayerController 0))))
      (Variables|Default|SetAs%20BP%20Base%20Hud _asbp_base_hud))))

(event EventTick
  (params (DeltaSeconds :type Float%20%28single-precision%29))
  (Utilities|FlowControl|Sequence
    (:then_0
      (CallFunction|UpdateTouchControls))
    (:then_1
      (CallFunction|UpdateOrientation))))

(event Input|ActionEvents|InputActionJump
  (params (Key :type Key%20Structure :default "None"))
  ;[1 1 1] PC controls
  (:Pressed
    (Character|Jump))
  (:Released
    (Character|StopJumping)))

(event Input|AxisEvents|InputAxisForward
  (params (AxisValue :type Float%20%28single-precision%29))
  ;[1 1 1] PC controls
  (Pawn|Input|AddMovementInput "0.000000,-1.000000,0.000000" AxisValue false)
  (Utilities|FlowControl|Gate true
    (:Exit
      (CallFunction|UpdateSpriteDirection AxisValue))))

(event Input|AxisEvents|InputAxisRight
  (params (AxisValue :type Float%20%28single-precision%29))
  ;[1 1 1] PC controls
  (Pawn|Input|AddMovementInput "1.000000,0.000000,0.000000" AxisValue false)
  (bind _bool (CallFunction|UpdateSpriteDirection AxisValue))
  (if _bool
    (Utilities|FlowControl|Gate true) ; enters at Close
    (else
      (Utilities|FlowControl|Gate true) ; enters at Open
    )))

(fn ConstructionScript)

(fn UpdateSpriteDirection
  (params (A :type Float%20%28double-precision%29))
  (bind _sprite (Variables|Default|GetSprite))
  (if (> (Math|Float|Absolute(Float) A) 0.0)
    (Utilities|FlowControl|Sequence
      (:then_0
        (if (> A 0.0)
          (Transformation|SetRelativeRotation _sprite "0.000000,-10.000000,-20.000000" false false)
          (else
            (Transformation|SetRelativeRotation _sprite "0.000000,170.000000,20.000000" false false))))
      (:then_1
        (return true)))
    (else
      (return false))))

(fn UpdateOrientation
  (Utilities|FlowControl|Sequence
    (:then_0
      (Variables|Default|SetCachedRotation (.yaw (Math|Rotator|MakeRotfromX (.Gravity (Class|PlayerController|GetInputMotionState (Game|GetPlayerController 0))))))
      (if (Math|Float|InRange(Float) (Variables|Default|GetCachedRotation) 6e+01 1.2e+02)
        (Variables|Default|SetOrientation "Portrait")
        (elif (Math|Float|InRange(Float) (Variables|Default|GetCachedRotation) -3e+01 3e+01)
          (Variables|Default|SetOrientation "LandscapeLeft")
          (elif (Math|Float|InRange(Float) (Variables|Default|GetCachedRotation) -1.2e+02 -6e+01)
            (Variables|Default|SetOrientation "PortraitUpsideDown")
            (elif (or (Math|Float|InRange(Float) (Variables|Default|GetCachedRotation) -1.9e+02 -1.5e+02) (Math|Float|InRange(Float) (Variables|Default|GetCachedRotation) 1.5e+02 1.9e+02))
              (Variables|Default|SetOrientation "LandscapeRight"))))))
    (:then_1
      (Variables|Default|SetOrientation "Portrait"))
    (:then_2
      (if (Utilities|Enum|NotEqual(Enum) (Variables|Default|GetPrevOrientation) (Variables|Default|GetOrientation))
        (Variables|Default|SetPrevOrientation (Variables|Default|GetOrientation))
        (CallFunction|OnOrientaionChanged (Variables|Default|GetOrientation))))))

(fn UpdateCameraOrientation
  (params (Orientation :type EScreenOrientation%20Enum :default "Unknown"))
  (bind _output_get (Variables|Default|SetA_TempCameraRot (Variables|/Script/Engine.SceneComponent|GetRelativeRotation (Variables|Default|GetCamera))))
  (Variables|Default|SetB_TempCameraRot (Math|Rotator|MakeRotator (Utilities|Select :Index Orientation :Unknown 0.0 :Portrait 0.0 :PortraitUpsideDown 1.8e+02 :LandscapeLeft 2.7e+02 :LandscapeRight 9e+01 :FaceUp 0.0 :FaceDown 0.0 :PortraitSensor 0.0 :LandscapeSensor 0.0 :FullSensor 0.0) (.Pitch (Math|Rotator|BreakRotator _output_get)) (.Yaw (Math|Rotator|BreakRotator _output_get))))
  (Components|Timeline|PlayfromStart (Variables|Default|GetOrientationChange)))