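; Base HUD Blueprint that draws simple screen-space lines and points from its variables.
; Each DrawHUD pass draws one thin line between DrawLineStart and DrawLineEnd.
; DrawPointCustom draws a small colored square for each entry in the DrawPointStart map, which pairs screen positions with colors.
; DrawPointCustom is not called within this Blueprint's own graphs.
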(event EventDrawHUD
  (params (SizeX :type Integer) (SizeY :type Integer))
  (bind _drawlinestart (Variables|Default|GetDrawLineStart))
  (bind _drawlineend (Variables|Default|GetDrawLineEnd))
  (Class|HUD|DrawLine (.x _drawlinestart) (.y _drawlinestart) (.x _drawlineend) (.y _drawlineend) "(R=0,G=0,B=0,A=1)" 1.0))

(fn ConstructionScript)

(fn DrawPointCustom
  (bind _drawpointstart (Variables|Default|GetDrawPointStart))
  (bind _keys (Utilities|Map|Keys _drawpointstart))
  (bind _values (Utilities|Map|Values _drawpointstart))
  (for (_array_element _array_index) _keys
    (HUD|DrawRect (Utilities|Array|Get(acopy) _values _array_index) (.X (Math|Vector|BreakVector _array_element)) (.Y (Math|Vector|BreakVector _array_element)) 5.0 5.0)))